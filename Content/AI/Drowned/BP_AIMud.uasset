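; AI controller for a mud enemy in the Drowned set that chooses its behavior tree from the boss's health when play begins.
; It finds the first Boss actor and truncates its health fraction times four into a quarter index.
; The middle two quarters run Mud3 and Mud2, while both the lowest quarter and the default, covering the top quarter, run Mud4.
; The choice is made once, with no later re-evaluation.
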(event `self.ReceiveBeginPlay`
  (bind _outactors (`GameplayStatics.GetAllActorsOfClass` "/Game/ThirdPersonCPP/Blueprints/Boss.Boss_C"))
  (bind _output (`|GetArrayItem` _outactors))
  (switch `int` (`KismetMathLibrary.FTrunc` (* (/ (`/Game/ThirdPersonCPP/Blueprints/Boss.CurrentHealth` _output) (`/Game/ThirdPersonCPP/Blueprints/Boss.MaxHealth` _output)) 4.0))
    (:`Default`
      (`self.RunBehaviorTree` "/Game/AI/Drowned/BT_Mud4.BT_Mud4"))
    (:`0`
      (`self.RunBehaviorTree` "/Game/AI/Drowned/BT_Mud4.BT_Mud4"))
    (:`1`
      (`self.RunBehaviorTree` "/Game/AI/Drowned/BT_Mud3.BT_Mud3"))
    (:`2`
      (`self.RunBehaviorTree` "/Game/AI/Drowned/BT_Mud2.BT_Mud2"))))

(fn `UserConstructionScript`)